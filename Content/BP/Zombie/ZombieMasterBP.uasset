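; Base zombie character for a horde shooter, with health, a punch attack and death handling.
; Attacks play a montage after a short delay, with damage left to an anim notify per the comment.
; Damage passes a not-dead check and updates the health text; death plays an animation, disables collision, sets a lifespan and rewards player 0's score.
; Destruction asks ZombieHordeGM_BP to check for the next round.
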(event `self.ReceiveBeginPlay`
  (`TextRenderComponent.K2_SetText` (`self.TextRender`) (`KismetTextLibrary.Conv_DoubleToText` (`self.Health`) "HalfToEven")))

(event `ZombieAttack`
  (params (Instigator :type "Controller Object Reference"))
  ;[1 0 0] Attack - Play montage // Damage from AnimNotifierHitboxDetection
  (`KismetSystemLibrary.Delay` 0.5)
  (if (not (`AnimInstance.IsAnyMontagePlaying` (`SkeletalMeshComponent.GetAnimInstance` (`self.Mesh`))))
    (`|PlayMontage` (`self.Mesh`) "/Game/Asset/Zombie/Animations/Maynard_punch_01_Montage.Maynard_punch_01_Montage" 1.5 0.5)))

(event `self.ReceiveAnyDamage`
  (params (Damage :type "Float (single-precision)") (DamageType :type "DamageType Object Reference") (InstigatedBy :type "Controller Object Reference") (DamageCauser :type "Actor Object Reference"))
  ;[1 1 1] Damage
  (`self.checkNotDead`
    (:`NotDead`
      (bind _output_get (set `self.Health` (`KismetMathLibrary.FClamp` (- (`self.Health`) Damage) 0.0 100.0)))
      (`TextRenderComponent.K2_SetText` (`self.TextRender`) (`KismetTextLibrary.Conv_DoubleToText` _output_get "HalfToEven"))
      (if (<= _output_get 0.0)
        (`self.OnDeath`)))))

(event `self.ReceiveDestroyed`
  ;[0 1 0.2331] Ask gamemode to check for next round
  (bind _aszombie_horde_gm_bp (cast `/Game/BP/Framework/ZombieHordeGM_BP` (`GameplayStatics.GetGameMode`)))
  (`/Game/BP/Framework/ZombieHordeGM_BP.CheckForNextRound` _aszombie_horde_gm_bp))

(fn `OnDeath`
  (set `self.isDead` true)
  (`|ExecutionSequence`
    (:`then_0`
      (`SkeletalMeshComponent.PlayAnimation` (`self.Mesh`) "/Game/Asset/Zombie/Animations/Maynard_death_02.Maynard_death_02" false)
      (`self.DetachFromControllerPendingDestroy`)
      (`PrimitiveComponent.SetCollisionEnabled` (`self.CapsuleComponent`) "NoCollision")
      (`SceneComponent.SetVisibility` (`self.TextRender`) false false)
      (`self.SetLifeSpan` 5.0))
    (:`then_1`
      ;[1 1 1] Add player kill reward
      (bind _ascoop_shooter_pc (cast `/Game/BP/Framework/CoopShooter_PC` (`GameplayStatics.GetPlayerController` 0)))
      (set `/Game/BP/Framework/CoopShooter_PC.Score` (+ (`/Game/BP/Framework/CoopShooter_PC.Score` _ascoop_shooter_pc) (`self.KillReward`)) _ascoop_shooter_pc))))

(fn `UserConstructionScript`)