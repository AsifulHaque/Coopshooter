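; Game mode for a round-based zombie horde game that runs wave progression and shop widgets.
; A looping countdown timer starts each round, telling every ZombieSpawner to spawn zombies with health and count scaled linearly by round.
; CheckForNextRound restarts the countdown when at most one zombie actor remains.
; It also creates the HUD and adds or removes vending machine and mystery box widgets, while ReqPurchase is a stub returning false.
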(event `self.ReceiveBeginPlay`
  ;[1 1 1] Widget to show Gamemode info
  (bind _returnvalue (`|CreateWidget` "/Game/UI/HUD_W.HUD_W_C" (`GameplayStatics.GetPlayerController` 0)))
  (`UserWidget.AddToViewport` _returnvalue 0)
  ;[1 1 1] Start first round
  (`self.StartNextRound`))

(event `/Game/BP/Framework/InteractableInterface.CreatePurchaseW`
  ;[1 1 1] Purchase Widget
  (bind _returnvalue (`|CreateWidget` "/Game/UI/PurchaseW.PurchaseW_C" (`GameplayStatics.GetPlayerController` 0)))
  (bind _output_get (set `self.VendingMachineUI` _returnvalue))
  (`UserWidget.AddToViewport` _output_get 0))

(event `/Game/BP/Framework/InteractableInterface.RemovePurchaseW`
  (bind _vendingmachineui (`self.VendingMachineUI`))
  ;[1 1 1] Remove Purchase W
  (`/Engine/EditorBlueprintResources/StandardMacros.IsValid` _vendingmachineui
    (:`Is Valid`
      (`Widget.RemoveFromParent` _vendingmachineui)
      (set `self.VendingMachineUI` null)
      (`WidgetBlueprintLibrary.SetInputMode_GameOnly` (`GameplayStatics.GetPlayerController` 0)))))

(event `/Game/BP/Framework/InteractableInterface.CreateMystBoxW`
  (params (OfferedItems :type "Array of /Game/BP/LevelAccessories/BuyableItemEnum Enum (by ref)" :default _))
  ;[1 1 1] Mystery box W
  (bind _returnvalue (`|CreateWidget` "/Game/UI/MysteryBoxW.MysteryBoxW_C" (`GameplayStatics.GetPlayerController` 0) OfferedItems))
  (bind _output_get (set `self.MysteryBoxW` _returnvalue))
  (`UserWidget.AddToViewport` _output_get 0))

(event `/Game/BP/Framework/InteractableInterface.RemoveMystBoxW`
  (bind _returnvalue (`GameplayStatics.GetPlayerController` 0))
  (bind _mysteryboxw (`self.MysteryBoxW`))
  ;[1 1 1] Remove Mystery Box
  (`/Engine/EditorBlueprintResources/StandardMacros.IsValid` _mysteryboxw
    (:`Is Valid`
      (`Widget.RemoveFromParent` _mysteryboxw)
      (set `self.MysteryBoxW` null)
      (set `PlayerController.bShowMouseCursor` false _returnvalue)
      (`WidgetBlueprintLibrary.SetInputMode_GameOnly` _returnvalue))))

(fn `CalculateZombieProperties`
  (returns (Health :type "Float (double-precision)") (NumOfZombie :type Integer))
  (bind _returnvalue (- (`self.Round`) 1))
  (return (+ (`KismetMathLibrary.Conv_IntToDouble` (* _returnvalue (`self.ZombieHealthIncreaseRate`))) (`self.BaseZombieHealth`)) (+ (* _returnvalue (`self.AdditionalZombiePerRound`)) (`self.BaseNumofZombie`))))

(fn `CheckForNextRound`
  (bind _outactors (`GameplayStatics.GetAllActorsOfClass` "/Game/BP/Zombie/ZombieMasterBP.ZombieMasterBP_C"))
  (if (not (`KismetArrayLibrary.Array_IsValidIndex` _outactors 1))
    (`self.StartNextRound`)))

(fn `Countdown`
  (bind _countdowntimerhandle (`self.CountDownTimerHandle`))
  (bind _output_get (set `self.CountDownTime` (- (`self.CountDownTime`) 1)))
  (if (== _output_get 0)
    (if (`KismetSystemLibrary.K2_IsValidTimerHandle` _countdowntimerhandle)
      (`KismetSystemLibrary.K2_ClearAndInvalidateTimerHandle` _countdowntimerhandle)
      (`self.NextRoundSpawn`))))

(fn `NextRoundSpawn`
  (`self.SpawnZombiesReq` (+ (`self.Round`) 1)))

(fn `ReqPurchase`
  (params (ItemToBuy :type "/Game/BP/LevelAccessories/BuyableItemEnum Enum" :default "NewEnumerator0") (Cost :type Integer))
  (returns (PurchaseSuccess :type Boolean))
  (return false))

(fn `SpawnZombiesReq`
  (params (Round :type Integer))
  (set `self.Round` Round)
  (bind (_health _numofzombie) (`self.CalculateZombieProperties`))
  (bind _outactors (`GameplayStatics.GetAllActorsOfClass` "/Game/BP/Zombie/ZombieSpawner.ZombieSpawner_C"))
  (for _array_element _outactors
    (`/Game/BP/Zombie/ZombieSpawner.spawnZombie` _array_element _health _numofzombie)))

(fn `StartNextRound`
  (set `self.CountDownTime` (`self.MaxCountdownTime`))
  (bind _returnvalue (`KismetSystemLibrary.K2_SetTimer` null "Countdown" 1.0 true 1.0))
  (set `self.CountDownTimerHandle` _returnvalue))

(fn `UserConstructionScript`)