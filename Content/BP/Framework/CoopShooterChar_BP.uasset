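; Player character Blueprint for a co-op shooter, extending a parent class with interaction and death-time prompt cleanup.
; Pressing Interact sends an interface message to every overlapping actor, so each one that implements it handles its own response.
; AnyDamage runs the parent logic first, then tells the game mode to remove the "purchase W" message if the character is dead.
; BeginPlay, Tick and construction only call the parent.
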(event `self.ReceiveBeginPlay`
  ;[1 1 1] Parent Functions
  (`parent.ReceiveBeginPlay`))

(event `self.ReceiveTick`
  (params (DeltaSeconds :type "Float (single-precision)"))
  ;[1 1 1] Parent Functions
  (`parent.ReceiveTick` DeltaSeconds))

(event `InputAction|Interact`
  (params (Key :type "Key Structure"))
  ;[1 1 1] Message overlapping interable actors that has interactable interface implemented
  (:`Pressed`
    (for _array_element (`self.GetOverlappingActors` null)
      (message `/Game/BP/Framework/InteractableInterface.Interact` _array_element))))

(event `self.ReceiveAnyDamage`
  (params (Damage :type "Float (single-precision)") (DamageType :type "DamageType Object Reference") (InstigatedBy :type "Controller Object Reference") (DamageCauser :type "Actor Object Reference"))
  ;[1 1 1] Remove if purchase W is showing
  (`parent.ReceiveAnyDamage` Damage DamageType InstigatedBy DamageCauser)
  (if (`self.IsDead`)
    (message `/Game/BP/Framework/InteractableInterface.RemovePurchaseW` (`GameplayStatics.GetGameMode`))))

(fn `UserConstructionScript`
  (`parent.UserConstructionScript`))