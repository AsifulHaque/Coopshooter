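; PlaceableDoorBP is a placeable door actor that takes damage and is destroyed when its health runs out.
; On BeginPlay it passes itself to its floating health bar widget as the parent actor.
; AnyDamage subtracts from a clamped DoorHealth and, on reaching zero, uses a short lifespan to remove the door after a brief delay.
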(event `self.ReceiveBeginPlay`
  ;[1 1 1] Set a ref to self in Widget
  (bind _asfoating_health_bar_w (cast `/Game/UI/FoatingHealthBarW` (`WidgetComponent.GetUserWidgetObject` (`self.Widget`))))
  (set `/Game/UI/FoatingHealthBarW.ParentActor` self _asfoating_health_bar_w))

(event `self.ReceiveAnyDamage`
  (params (Damage :type "Float (single-precision)") (DamageType :type "DamageType Object Reference") (InstigatedBy :type "Controller Object Reference") (DamageCauser :type "Actor Object Reference"))
  (bind _doorhealth (`self.DoorHealth`))
  ;[1 1 1] Damage
  (if (> _doorhealth 0.0)
    (bind _output_get (set `self.DoorHealth` (`KismetMathLibrary.FClamp` (- _doorhealth Damage) 0.0 100.0)))
    (if (== _output_get 0.0)
      (`self.SetLifeSpan` 1.0))))

(fn `UserConstructionScript`)