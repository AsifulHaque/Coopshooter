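; Vending machine actor placed in levels that the player can approach and interact with to open a purchase UI.
; A text prompt shows while the player pawn overlaps it and hides on exit, which also clears the purchase message through the game mode.
; Interact asks the game mode to create that purchase message when no VendingMachineUI is valid.
; ReqPurchase is a stub that always returns false.
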(event `self.ReceiveActorBeginOverlap`
  (params (OtherActor :type "Actor Object Reference"))
  ;[1 1 1] Show Hide UI text
  (if (== OtherActor (`GameplayStatics.GetPlayerPawn` 0))
    (`SceneComponent.SetVisibility` (`self.TextRender`) true false)))

(event `self.ReceiveActorEndOverlap`
  (params (OtherActor :type "Actor Object Reference"))
  ;[1 1 1] Show Hide UI text
  (if (== OtherActor (`GameplayStatics.GetPlayerPawn` 0))
    (`SceneComponent.SetVisibility` (`self.TextRender`) false false)
    ;[1 1 1] Clear and reset the UI
    (message `/Game/BP/Framework/InteractableInterface.RemovePurchaseW` (`GameplayStatics.GetGameMode`))))

(event `/Game/BP/Framework/InteractableInterface.Interact`
  ;[1 1 1] Interact Call from player
  (`/Engine/EditorBlueprintResources/StandardMacros.IsValid` (`self.VendingMachineUI`)
    (:`Is Not Valid`
      (message `/Game/BP/Framework/InteractableInterface.CreatePurchaseW` (`GameplayStatics.GetGameMode`)))))

(fn `ReqPurchase`
  (params (ItemToBuy :type "/Game/BP/LevelAccessories/BuyableItemEnum Enum" :default "NewEnumerator0") (Cost :type Integer))
  (returns (PurchaseSuccess :type Boolean))
  (return false))

(fn `UserConstructionScript`)