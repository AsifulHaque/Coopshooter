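; MysteryBoxBP is an interactable mystery box placed in levels that offers the player a set of possible items.
; Its text label shows while the player pawn overlaps it and hides on exit, which also removes any open mystery box widget.
; Interacting has the game mode create that widget from the box's PossibleItems list.
; Its ReqPurchase function is a stub that always returns false.
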(event `self.ReceiveActorBeginOverlap`
  (params (OtherActor :type "Actor Object Reference"))
  ;[1 1 1] Show Hide UI text
  (if (== OtherActor (`GameplayStatics.GetPlayerPawn` 0))
    (`SceneComponent.SetVisibility` (`self.TextRender`) true false)))

(event `self.ReceiveActorEndOverlap`
  (params (OtherActor :type "Actor Object Reference"))
  ;[1 1 1] Show Hide UI text
  (if (== OtherActor (`GameplayStatics.GetPlayerPawn` 0))
    (`SceneComponent.SetVisibility` (`self.TextRender`) false false)
    ;[1 1 1] Remove mysterybox Widget if any
    (message `/Game/BP/Framework/InteractableInterface.RemoveMystBoxW` (`GameplayStatics.GetGameMode`))))

(event `/Game/BP/Framework/InteractableInterface.Interact`
  ;[1 1 1] Create MystBoxW on interact
  (message `/Game/BP/Framework/InteractableInterface.CreateMystBoxW` (`GameplayStatics.GetGameMode`) (`self.PossibleItems`)))

(fn `ReqPurchase`
  (params (ItemToBuy :type "/Game/BP/LevelAccessories/BuyableItemEnum Enum" :default "NewEnumerator0") (Cost :type Integer))
  (returns (PurchaseSuccess :type Boolean))
  (return false))

(fn `UserConstructionScript`)